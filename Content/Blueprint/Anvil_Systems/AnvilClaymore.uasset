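; Anvil display claymore that shows itself only while the player's DummyCharacter has the claymore selected (WeaponId 3).
; Each Tick reads the player pawn's WeaponId and toggles the main static mesh's visibility to match.
; The Visibility function, also run on Tick and mirrored in the construction script, copies that state to the Crossguard, Pommel and Hilt meshes.
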(event EventTick
  (params (DeltaSeconds :type Float%20%28single-precision%29))
  (CallFunction|Visibility)
  (bind _asdummy_character (Utilities|Casting|CastToDummyCharacter (Game|Player|GetPlayerPawn 0)))
  (Math|Integer|CompareInt (Variables|/Game/Blueprint/DummyCharacter.DummyCharacter_C|GetWeaponId _asdummy_character) 3
    (:>
      (Rendering|SetVisibility (Variables|Debug|GetStaticMeshComponent) false false :!label _label))
    (:==
      (Rendering|SetVisibility (Variables|Debug|GetStaticMeshComponent) true false))
    (:<
      (goto _label))))

(fn ConstructionScript
  (if (Rendering|IsVisible (Variables|Debug|GetStaticMeshComponent))
    (Rendering|SetVisibility (Variables|Default|Getcrossguard) true false)
    (else
      (Rendering|SetVisibility (Variables|Default|Getcrossguard) false false))))

(fn Visibility
  ;[1 1 1] This line of blueprint ensures that if the claymores visibility is toggled, every static mesh component of the claymore has it's visibility toggled too
  (if (Rendering|IsVisible (Variables|Debug|GetStaticMeshComponent))
    (Rendering|SetVisibility (Variables|Default|Getcrossguard) true false)
    (else
      (Rendering|SetVisibility (Variables|Default|Getcrossguard) false false))))