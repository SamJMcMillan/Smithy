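; DummyCharacter is a Blueprint that holds shared state and widgets for a weapon-forging order system.
; On BeginPlay it creates the mines menu and anvil crafting widgets for access via casting, loads OrdersTable rows into an array and picks three random available orders.
; Lookup functions turn numeric Vector2D components into metal and weapon type names.
; Pressing K opens a delete-save confirmation widget.
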(event EventBeginPlay
  ;[0.156 1 0.8194] These nodes prepare the max size of the CurrentOrders array
  (Utilities|Array|Resize (Variables|Default|GetCurrentOrders) 3)
  ;[0.3127 0 1] These widgets need to be referenced elsewhere, so they are created in DummyCharacter so that they can be easily casted to
  (bind _returnvalue (UserInterface|CreateWidget "/Game/Interface/Mines_Menu.Mines_Menu_C"))
  (Variables|Default|SetMines_Menu _returnvalue)
  (bind _returnvalue_2 (UserInterface|CreateWidget "/Game/Interface/AnvilCrafting.AnvilCrafting_C"))
  (Variables|Default|SetAnvilCrafting _returnvalue_2)
  (Input|EnableInput 0)
  ;[0 1 0.9261] This line of blueprint creates the OrderStructureArray
  (bind _outrownames (DataTable|GetDataTableRowNames "/Game/Blueprint/Orders_System/OrdersTable.OrdersTable"))
  (for _array_element _outrownames
    (bind _returnvalue_3 (Utilities|GetDataTableRow "/Game/Blueprint/Orders_System/OrdersTable.OrdersTable" _array_element)
      (:then
        (Utilities|Array|Add (Variables|Default|GetOrderStructureArray) _returnvalue_3))))
  ;[0 1 0.195] Order Randomiser
  (for _index (range 0 2)
    (bind _selectedorder (CallFunction|GetRandomOrder (Variables|Default|GetOrderStructureArray)))
    (Utilities|Array|Add (Variables|Default|GetCurrentlyAvailableOrders) _selectedorder)))

(event Input|KeyboardEvents|K
  (params (Key :type Key%20Structure))
  (:Pressed
    (bind _returnvalue (UserInterface|CreateWidget "/Game/Interface/Interface_Misc/DeleteSave_Sure.DeleteSave_Sure_C"))
    (UserInterface|Viewport|AddtoViewport _returnvalue 0)))

(fn ConstructionScript)

(fn GetRandomOrder
  (params (OrderStructureArrayRef :type Array%20of%20Orders%20Structure%20Structures))
  (return (Utilities|Array|Get(acopy) OrderStructureArrayRef (Math|Random|RandomIntegerinRange 0 (- (Utilities|Array|Length OrderStructureArrayRef) 1)))))

(fn WeaponMetalLookUp
  (params (X :type Float%20%28single-precision%29))
  (bind _returnvalue (Math|Float|Truncate X))
  ;[0 0.9605 1] This funtion allows us to display the metal names assigned to Vector2D values
  (if (== _returnvalue 1)
    (LocalVariables|SetMetalNameLocalRef "Bronze")
    (return (LocalVariables|GetMetalNameLocalRef))
    (elif (== _returnvalue 2)
      (LocalVariables|SetMetalNameLocalRef "Iron")
      (return (LocalVariables|GetMetalNameLocalRef))
      (elif (== _returnvalue 3)
        (LocalVariables|SetMetalNameLocalRef "Steel")
        (return (LocalVariables|GetMetalNameLocalRef))
        (elif (== _returnvalue 4)
          (LocalVariables|SetMetalNameLocalRef "Silver")
          (return (LocalVariables|GetMetalNameLocalRef))
          (elif (== _returnvalue 5)
            (LocalVariables|SetMetalNameLocalRef "Gold")
            (return (LocalVariables|GetMetalNameLocalRef))))))))

(fn WeaponTypeLookUp
  (params (Y :type Float%20%28single-precision%29))
  (bind _returnvalue (Math|Float|Truncate Y))
  (if (== _returnvalue 1)
    (LocalVariables|SetLocalWeaponTypeRef "Longsword")
    (return (LocalVariables|GetLocalWeaponTypeRef))
    (elif (== _returnvalue 2)
      (LocalVariables|SetLocalWeaponTypeRef "Polearm")
      (return (LocalVariables|GetLocalWeaponTypeRef))
      (elif (== _returnvalue 3)
        (LocalVariables|SetLocalWeaponTypeRef "Claymore")
        (return (LocalVariables|GetLocalWeaponTypeRef))
        (elif (== _returnvalue 4)
          (LocalVariables|SetLocalWeaponTypeRef "Greataxe")
          (return (LocalVariables|GetLocalWeaponTypeRef))
          (elif (== _returnvalue 5)
            (LocalVariables|SetLocalWeaponTypeRef "Warhammer")
            (return (LocalVariables|GetLocalWeaponTypeRef))))))))